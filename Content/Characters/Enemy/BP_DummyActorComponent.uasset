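; A health-bar widget component that gives its owning dummy enemy health, damage handling and death.
; It binds to the owner's overlap event, subtracting and destroying any Jungle_Bullet that hits, and also accepts damage through ApplyDamage.
; Health changes update BP_DummyWidget, which turns toward the player's pawn each tick.
; At zero health it spawns an explosion and destroys the owner.
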(event `self.ReceiveBeginPlay`
  (bind _returnvalue (`self.GetOwner`))
  (if (`KismetSystemLibrary.IsValid` _returnvalue)
    (add `Actor.OnActorBeginOverlap` _returnvalue (delegate `OnOverlapHandler`))
    (set `self.Health` (`self.MaxHealth`))
    (`self.UpdateHealthValue`)))

(event `OnOverlapHandler`
  (params (OverlappedActor :type "Actor Object Reference") (OtherActor :type "Actor Object Reference"))
  (`self.OverlapHandler` OtherActor))

(event `UpdateHealthValue`
  (bind _asbp_dummy_widget (cast `/Game/Characters/Enemy/BP_DummyWidget` (`self.GetUserWidgetObject`)))
  (`/Game/Characters/Enemy/BP_DummyWidget.SetNewHelthValue` _asbp_dummy_widget (/ (`self.Health`) (`self.MaxHealth`))))

(event `self.ReceiveTick`
  (params (DeltaSeconds :type "Float (single-precision)"))
  (`self.K2_SetWorldRotation` (`KismetMathLibrary.FindLookAtRotation` (`self.K2_GetComponentLocation`) (`Actor.K2_GetActorLocation` (`Controller.K2_GetPawn` (`GameplayStatics.GetPlayerController` 0))))))

(event `OverlapHandler`
  (params (`Overlaped Actor` :type "Actor Object Reference"))
  (bind _asjungle_bullet (cast `Jungle_Bullet` `Overlaped Actor`))
  (bind _output_get (set `self.Health` (- (`self.Health`) (`Jungle_Bullet.Damage` _asjungle_bullet))))
  (bind _output_get_2 (set `self.Projectile Location` (`Actor.K2_GetActorLocation` _asjungle_bullet)))
  (`Actor.K2_DestroyActor` _asjungle_bullet)
  (if (<= _output_get 0.0)
    (`self.DestroyActorHandler` _output_get_2)
    (else
      (`self.UpdateHealthValue`))))

(event `DestroyActorHandler`
  (params (ProjectileLocation :type "Vector Structure"))
  (bind _returnvalue (`self.GetOwner`))
  (if (`KismetSystemLibrary.IsValid` _returnvalue)
    (`GameplayStatics.SpawnEmitterAtLocation` "/MultiplayerFPS/ParticleEffects/P_Explosion.P_Explosion" (`Actor.K2_GetActorLocation` _returnvalue))
    (`Actor.K2_DestroyActor` (`self.GetOwner`))
    (else
      (`GameplayStatics.SpawnEmitterAtLocation` "/MultiplayerFPS/ParticleEffects/P_Explosion.P_Explosion" ProjectileLocation))))

(event `ApplyDamage`
  (params (Damage :type "Float (double-precision)"))
  (bind _output_get (set `self.Health` (- (`self.Health`) Damage)))
  (if (<= _output_get 0.0)
    (`self.DestroyActorHandler` (0.0 0.0 0.0))
    (else
      (`self.UpdateHealthValue`))))